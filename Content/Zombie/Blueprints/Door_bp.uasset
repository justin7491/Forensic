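; Door Blueprint that the player swings open or shut by holding the Drag Door input.
; On press, a short line trace from the player camera enables dragging if it hits any Door_bp, not specifically this instance.
; While dragging, Tick yaws the door by the player's TurnRate times Sensitivity.
; A world-yaw check against Openangel snaps it just inside the limit using relative rotation.
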(event `self.ReceiveTick`
  (params (DeltaSeconds :type "Float (single-precision)"))
  (bind _openangel (`self.Openangel`))
  (bind _openangel_2 (`self.Openangel`))
  (bind _door (`self.Door`))
  (bind (_returnvalue_roll _returnvalue_pitch _returnvalue_yaw) (`KismetMathLibrary.BreakRotator` (`SceneComponent.K2_GetComponentRotation` (`self.Door`))))
  (if (`self.IsHoldingLMB?`)
    (if (`self.IsLookingAt?`)
      (if (not (== _returnvalue_yaw (`KismetMathLibrary.ClampAngle` _returnvalue_yaw _openangel (* _openangel -1.0))))
        (`SceneComponent.K2_AddLocalRotation` _door (`KismetMathLibrary.MakeRotator` 0.0 0.0 (* (`/Game/Zombie/Blueprints/bp_player.Turn Rate` (stale `InputAction|Drag Door` _asbp_player)) (`self.Sensitivity`))) false false)
        (elif (>= _returnvalue_yaw _openangel_2)
          (`SceneComponent.K2_SetRelativeRotation` _door (`KismetMathLibrary.MakeRotator` 0.0 0.0 (- _openangel_2 1.0)) false false)
          (else
            (`SceneComponent.K2_SetRelativeRotation` _door (`KismetMathLibrary.MakeRotator` 0.0 0.0 (+ (* _openangel_2 -1.0) 1.0)) false false)))))))

(event `self.ReceiveBeginPlay`
  (`self.EnableInput` (`GameplayStatics.GetPlayerController` 0)))

(event `InputAction|Drag Door`
  (params (Key :type "Key Structure"))
  (:`Pressed`
    (set `self.IsHoldingLMB?` true)
    (bind _asbp_player (cast `/Game/Zombie/Blueprints/bp_player` (`GameplayStatics.GetPlayerCharacter` 0)))
    (bind _fpc (`/Game/Zombie/Blueprints/bp_player.FPC` _asbp_player))
    (bind _returnvalue (`SceneComponent.K2_GetComponentLocation` _fpc))
    (bind (_outhit _returnvalue_2) (`KismetSystemLibrary.LineTraceSingleForObjects` :`Start` _returnvalue :`End` (+ _returnvalue (* (`SceneComponent.GetForwardVector` _fpc) 100.0)) :`ObjectTypes` (`|MakeArray` "ObjectTypeQuery2" :!type "EObjectTypeQuery Enum") :`bIgnoreSelf` false))
    (if _returnvalue_2
      (cast `/Game/Zombie/Blueprints/Door_bp` (`.HitActor` (`GameplayStatics.BreakHitResult` _outhit)))
      (set `self.IsLookingAt?` true)
      (else
        (set `self.IsLookingAt?` false))))
  (:`Released`
    (set `self.IsLookingAt?` false)))

(fn `UserConstructionScript`)