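; First-person player character Blueprint handling movement, mouse look, sprint, toggle crouch, zoom, flashlight and pause menu.
; Tick drives speed-based walk/run camera shakes, aligns the spotlight with control rotation, and drains or regenerates stamina through one-second Delays.
; Sprint changes walk speed and ends when stamina runs out.
; A timeline animates zoom FOV, and FlipFlops toggle crouch and the pause widget; controller-sensitivity look nodes are left unwired.
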(event `self.ReceiveTick`
  (params (DeltaSeconds :type "Float (single-precision)"))
  (`self.Headbob`)
  (`SceneComponent.K2_SetWorldRotation` (`self.SpotLight`) (`self.GetControlRotation`) false false)
  (if (`self.Is Sprinting?`)
    (`KismetSystemLibrary.Delay` 1.0)
    (if (<= (`self.Stamina`) 0)
      (set `self.Is Sprinting?` false)
      (set `CharacterMovementComponent.MaxWalkSpeed` 450.0 (`self.CharacterMovement`))
      (else
        (set `self.Stamina` (- (`self.Stamina`) 10))))
    (else
      (`KismetSystemLibrary.Delay` 1.0)
      (if (< (`self.Stamina`) (`self.Max Stamina`))
        (set `self.Stamina` (+ (`self.Stamina`) 5))))))

(event `InputAction|zoom`
  (params (Key :type "Key Structure"))
  (:`Pressed`
    (set `self.iszoom?` true)
    (bind (_direction _zoom) (`Timeline|Zoom` :!label _label)
      (:`Update`
        (`CameraComponent.SetFieldOfView` (`self.FPC`) _zoom))))
  (:`Released`
    (set `self.iszoom?` false)
    (goto _label :!via `Reverse`)))

(event `Headbob`
  (bind _returnvalue (`GameplayStatics.GetPlayerController` 0))
  (bind _returnvalue_2 (`KismetMathLibrary.VSize` (`self.GetVelocity`)))
  (if (and (> _returnvalue_2 0.0) (`self.CanJump`))
    (if (< _returnvalue_2 500.0)
      (`PlayerController.ClientStartCameraShakeFromSource` _returnvalue "/Game/Zombie/Blueprints/Walk.Walk_C" null)
      (else
        (`PlayerController.ClientStartCameraShakeFromSource` _returnvalue "/Game/Zombie/Blueprints/Run.Run_C" null)))))

(event `InputAction|Sprint`
  (params (Key :type "Key Structure"))
  ;[1 1 1] basic movement
  (:`Pressed`
    (if (>= (`self.Stamina`) 1)
      (set `self.Is Sprinting?` true)
      (set `CharacterMovementComponent.MaxWalkSpeed` 1000.0 (`self.CharacterMovement`))))
  (:`Released`
    (set `CharacterMovementComponent.MaxWalkSpeed` 450.0 (`self.CharacterMovement`))
    (set `self.Is Sprinting?` false)))

(event `InputAxis|Move Forward`
  (params (AxisValue :type "Float (single-precision)"))
  (bind (_returnvalue_roll _returnvalue_pitch _returnvalue_yaw) (`KismetMathLibrary.BreakRotator` (`self.GetControlRotation`)))
  ;[1 1 1] basic movement
  (`self.AddMovementInput` (`KismetMathLibrary.GetForwardVector` (`KismetMathLibrary.MakeRotator` 0.0 0.0 _returnvalue_yaw)) AxisValue))

(event `InputAxis|Move Backwards`
  (params (AxisValue :type "Float (single-precision)"))
  (bind (_returnvalue_roll _returnvalue_pitch _returnvalue_yaw) (`KismetMathLibrary.BreakRotator` (`self.GetControlRotation`)))
  ;[1 1 1] basic movement
  (`self.AddMovementInput` (`KismetMathLibrary.GetForwardVector` (`KismetMathLibrary.MakeRotator` 0.0 0.0 _returnvalue_yaw)) AxisValue))

(event `InputAction|Crouch`
  (params (Key :type "Key Structure"))
  ;[1 1 1] basic movement
  (:`Pressed`
    (`/Engine/EditorBlueprintResources/StandardMacros.FlipFlop`
      (:`A`
        (`self.Crouch`)
        (set `self.iscrouching?` true))
      (:`B`
        (`self.UnCrouch`)
        (set `self.iscrouching?` false)))))

(event `InputAxis|Move Left`
  (params (AxisValue :type "Float (single-precision)"))
  (bind (_returnvalue_roll _returnvalue_pitch _returnvalue_yaw) (`KismetMathLibrary.BreakRotator` (`self.GetControlRotation`)))
  ;[1 1 1] basic movement
  (`self.AddMovementInput` (`KismetMathLibrary.GetRightVector` (`KismetMathLibrary.MakeRotator` 0.0 0.0 _returnvalue_yaw)) AxisValue))

(event `InputAxis|Mouse Look Horizontal`
  (params (AxisValue :type "Float (single-precision)"))
  ;[1 1 1] basic movement
  (`self.AddControllerYawInput` (* AxisValue (`self.Mouse Sensitivity`) (`GameplayStatics.GetWorldDeltaSeconds`)))
  (set `self.Turn Rate` AxisValue))

(event `InputAxis|Move Right`
  (params (AxisValue :type "Float (single-precision)"))
  (bind (_returnvalue_roll _returnvalue_pitch _returnvalue_yaw) (`KismetMathLibrary.BreakRotator` (`self.GetControlRotation`)))
  ;[1 1 1] basic movement
  (`self.AddMovementInput` (`KismetMathLibrary.GetRightVector` (`KismetMathLibrary.MakeRotator` 0.0 0.0 _returnvalue_yaw)) AxisValue))

(event `InputAxis|Mouse Look Vertical`
  (params (AxisValue :type "Float (single-precision)"))
  ;[1 1 1] basic movement
  (`self.AddControllerPitchInput` (* AxisValue (`self.Mouse Sensitivity`) (`GameplayStatics.GetWorldDeltaSeconds`))))

(event `InputAction|Flashlight`
  (params (Key :type "Key Structure"))
  ;[1 1 1] Toggle On/Off Flashlight
  (:`Pressed`
    (if (`self.isflashlighton?`)
      (`GameplayStatics.PlaySound2D` "/Game/Zombie/Audio/Flashlight_Off.Flashlight_Off" 0.2 1.0 0.0 null null)
      (`self.TurnFlashlightOff`)
      (else
        (`GameplayStatics.PlaySound2D` "/Game/Zombie/Audio/Flashlight_On.Flashlight_On" 0.1 1.0 0.0 null null)
        (`self.TurnFlashlightON`)))))

(event `InputAction|Pause` :paused true
  (params (Key :type "Key Structure"))
  (bind _returnvalue (`GameplayStatics.GetPlayerController` 0))
  ;[1 1 1] Pause
  (:`Pressed`
    (`/Engine/EditorBlueprintResources/StandardMacros.FlipFlop`
      (:`A`
        (bind _returnvalue_2 (`|CreateWidget` "/Game/Zombie/Pause_Menu/PauseMenuWidget.PauseMenuWidget_C"))
        (`UserWidget.AddToViewport` _returnvalue_2 0)
        (`GameplayStatics.SetGamePaused` true)
        (set `PlayerController.bShowMouseCursor` true _returnvalue))
      (:`B`
        (`Widget.RemoveFromParent` _returnvalue_2)
        (`GameplayStatics.SetGamePaused` false)
        (set `PlayerController.bShowMouseCursor` false _returnvalue)))))

(fn `TurnFlashlightOff`
  (`SceneComponent.SetVisibility` (`self.SpotLight`) false false)
  (set `self.isflashlighton?` false))

(fn `TurnFlashlightON`
  (`SceneComponent.SetVisibility` (`self.SpotLight`) true false)
  (set `self.isflashlighton?` true))

(fn `UserConstructionScript`)